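; Player character paired with a LittleCube companion, spawned at BeginPlay to follow a FollowPoint that flips against X velocity.
; ToggleTotem attaches or detaches the cube at the totem point, or, once launched, stops its physics and moves it to world origin.
; ThrowEvent launches an attached cube by physics impulse, directed by Y velocity.
; Move remaps input axes using collider flags, and two events play top-down and 2D view sequences.
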(event `self.ReceiveTick`
  (params (DeltaSeconds :type "Float (single-precision)"))
  ;[0.02956 0.07421 0.1119] EventTick
  (if (> 0.0 (.x (`self.GetVelocity`)))
    (`SceneComponent.K2_SetRelativeLocation` (`self.FollowPoint`) (150.0 0.0 0.0) false true)
    (else
      (`SceneComponent.K2_SetRelativeLocation` (`self.FollowPoint`) (-150.0 0.0 0.0) false true))))

(event `Move`
  (params (X :type "Float (double-precision)") (Y :type "Float (double-precision)"))
  ;[0.02217 0.04519 0.06301] Mouvement
  (if (`self.PassIncollider`)
    (if (`self.ChangeInput`)
      (`self.AddMovementInput` (`self.GetActorRightVector`) X)
      (`self.AddMovementInput` (`self.GetActorForwardVector`) Y)
      (`KismetSystemLibrary.PrintString` "Change")
      (else
        (`KismetSystemLibrary.PrintString` "ManqueChangeInput")))
    (else
      (`self.AddMovementInput` (`self.GetActorRightVector`) Y)
      (`self.AddMovementInput` (`self.GetActorForwardVector`) X))))

(event `ThrowEvent`
  ;[0.04971 0.1022 0.147] CallThrowEvent
  (`self.Throw`))

(event `InputAction|ToggleTotem`
  (params (Key :type "Key Structure"))
  (bind _littlecubemesh (`/Game/Blueprints/LittleBrother/BP_LittleCube.LittleCubeMesh` (`self.LittleCubeRef`)))
  ;[0.0319 0.0648 0.0865] TotemInputAction
  (:`Pressed`
    (if (`/Game/Blueprints/LittleBrother/BP_LittleCube.IsLaunched` (`self.LittleCubeRef`))
      (`PrimitiveComponent.SetSimulatePhysics` _littlecubemesh false)
      (`PrimitiveComponent.SetEnableGravity` _littlecubemesh false)
      (`self.K2_SetActorLocation` (`self.LittleCubeRef`) (0.0 0.0 0.0) false false)
      (set `/Game/Blueprints/LittleBrother/BP_LittleCube.OnTotem` false (`self.LittleCubeRef`))
      (set `/Game/Blueprints/LittleBrother/BP_LittleCube.IsLaunched` false (`self.LittleCubeRef`))
      (elif (`self.TotemActive`)
        (`KismetSystemLibrary.PrintString` "Detach")
        (`self.Detach`)
        (else
          (`KismetSystemLibrary.PrintString` "Attach")
          (`self.Attach`))))))

(event `TopDownLake`
  ;[0.1559 0.02029 0.01938] ActorSequencer
  (`ActorSequenceComponent.PlaySequence` (`self.ViewTopDown`)))

(event `2DViewForest`
  ;[0.1559 0.02029 0.01938] ActorSequencer
  (`ActorSequenceComponent.PlaySequence` (`self.2DView`)))

(event `self.ReceiveBeginPlay`
  ;[0.0319 0.0648 0.09306] SetupSpawnParentCube
  (bind _returnvalue (`|SpawnActorFromClass` "/Game/Blueprints/LittleBrother/BP_LittleCube.BP_LittleCube_C" (`KismetMathLibrary.MakeTransform` (+ (`self.K2_GetActorLocation`) (`KismetMathLibrary.MakeVector` -150.0))) "Undefined" "MultiplyWithRoot" null self null))
  (bind _output_get (set `self.LittleCubeRef` _returnvalue))
  (set `/Game/Blueprints/LittleBrother/BP_LittleCube.FollowTarget` (`self.FollowPoint`) _output_get)
  (`KismetSystemLibrary.PrintString` "Spawn OK")
  (set `/Game/Blueprints/LittleBrother/BP_LittleCube.BigCubeRef` (`self.BigCubeRef`) _returnvalue))

(fn `Attach`
  (bind _littlecuberef (`self.LittleCubeRef`))
  ;[0.1119 0.02029 0.1529] Attach
  (`self.K2_SetActorLocation` _littlecuberef (`SceneComponent.K2_GetComponentLocation` (`self.AttachTotemPoint`)) false true)
  (`self.K2_AttachToComponent` _littlecuberef (`self.AttachTotemPoint`) "None" "SnapToTarget" "SnapToTarget" "KeepWorld" true)
  (`KismetSystemLibrary.PrintString` "C'est attaché")
  (set `self.TotemActive` true)
  (set `/Game/Blueprints/LittleBrother/BP_LittleCube.OnTotem` true (`self.LittleCubeRef`)))

(fn `Detach`
  ;[0.1329 0.02956 0.1746] Detach
  (`self.K2_SetActorLocation` (`self.LittleCubeRef`) (`SceneComponent.K2_GetComponentLocation` (`self.AttachTotemPoint`)) false true)
  (`self.K2_DetachFromActor` "KeepWorld" "KeepWorld" "KeepWorld")
  (`KismetSystemLibrary.PrintString` "C'est déttaché")
  (set `self.TotemActive` false)
  (set `/Game/Blueprints/LittleBrother/BP_LittleCube.OnTotem` false (`self.LittleCubeRef`)))

(fn `Throw`
  (bind _littlecuberef (`self.LittleCubeRef`))
  (bind _littlecubemesh (`/Game/Blueprints/LittleBrother/BP_LittleCube.LittleCubeMesh` (`self.LittleCubeRef`)))
  ;[0.1195 0.02122 0.162] Throw
  (if (`/Game/Blueprints/LittleBrother/BP_LittleCube.OnTotem` (`self.LittleCubeRef`))
    (`self.K2_DetachFromActor` (`self.LittleCubeRef`) "KeepWorld" "KeepWorld" "KeepWorld")
    (`PrimitiveComponent.SetSimulatePhysics` _littlecubemesh true)
    (`PrimitiveComponent.SetEnableGravity` _littlecubemesh true)
    (`PrimitiveComponent.AddImpulse` (`/Game/Blueprints/LittleBrother/BP_LittleCube.LittleCubeMesh` (`self.LittleCubeRef`)) (`KismetMathLibrary.SelectVector` (1000.0 0.0 400.0) (-1000.0 0.0 400.0) (> (.y (`self.GetVelocity`)) 0.0)) "None" true)
    (set `/Game/Blueprints/LittleBrother/BP_LittleCube.IsLaunched` true _littlecuberef)
    (set `/Game/Blueprints/LittleBrother/BP_LittleCube.OnTotem` false _littlecuberef)))

(fn `UserConstructionScript`)
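; BP_LittleCube is a cube actor in the LittleBrother folder that trails a follow target.
; Each tick, while it is neither on a totem nor launched and the target is valid, it interpolates toward that scene component's world location.
; It moves by teleporting without sweep, so the follow motion ignores collision.
; The totem and launch states are only read here, never set.
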(event `self.ReceiveTick`
  (params (DeltaSeconds :type "Float (single-precision)"))
  (bind _followtarget (`self.FollowTarget`))
  (if (and (not (`self.OnTotem`)) (not (`self.IsLaunched`)))
    (`/Engine/EditorBlueprintResources/StandardMacros.IsValid` _followtarget
      (:`Is Valid`
        (`self.K2_SetActorLocation` (`KismetMathLibrary.VInterpTo` (`self.K2_GetActorLocation`) (`SceneComponent.K2_GetComponentLocation` _followtarget) DeltaSeconds 10.0) false true)))))

(fn `UserConstructionScript`)